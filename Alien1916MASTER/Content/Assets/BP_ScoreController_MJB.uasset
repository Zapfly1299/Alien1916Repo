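; BP_ScoreController_MJB tracks the player's score and applies a time-based multiplier to points earned.
; From BeginPlay, a chain of delays changes ScoreModifier over three minutes, first raising it, then stepping it down in stages.
; AddScore multiplies incoming points by the current modifier and adds the result to CurrentScore.
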(event `self.ReceiveBeginPlay`
  (`KismetSystemLibrary.Delay` 30.0)
  (set `self.ScoreModifier` 1.5)
  (`KismetSystemLibrary.Delay` 30.0)
  (set `self.ScoreModifier` 1.0)
  (`KismetSystemLibrary.Delay` 60.0)
  (set `self.ScoreModifier` 0.75)
  (`KismetSystemLibrary.Delay` 60.0)
  (set `self.ScoreModifier` 0.5))

(fn `AddScore`
  (params (ScoreToAdd :type "Float (double-precision)"))
  (set `self.CurrentScore` (+ (* ScoreToAdd (`self.ScoreModifier`)) (`self.CurrentScore`))))

(fn `UserConstructionScript`)