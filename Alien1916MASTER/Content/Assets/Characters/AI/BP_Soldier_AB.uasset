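; AI soldier character that fires projectiles at the player and exposes a setter for its walk speed.
; SoldierShoot spawns a BP_Bullet_AB at ShootLocation, rotated toward the player pawn with a fixed yaw offset, then adds ProjectileVelocity to its velocity in local space.
; UpdateWalkSpeed writes the character movement's max walk speed; neither it nor SoldierShoot is called within this Blueprint.
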(event `SoldierShoot`
  (bind _shootlocation (`self.ShootLocation`))
  (bind (_returnvalue_roll _returnvalue_pitch _returnvalue_yaw) (`KismetMathLibrary.BreakRotator` (`KismetMathLibrary.FindLookAtRotation` (`SceneComponent.K2_GetComponentLocation` _shootlocation) (`self.K2_GetActorLocation` (`GameplayStatics.GetPlayerPawn` 0)))))
  (bind _returnvalue (`|SpawnActorFromClass` "/Game/Assets/Characters/AI/BP_Bullet_AB.BP_Bullet_AB_C" (`KismetMathLibrary.MakeTransform` (`SceneComponent.K2_GetComponentLocation` _shootlocation) (`KismetMathLibrary.MakeRotator` _returnvalue_roll _returnvalue_pitch (- _returnvalue_yaw 35.0))) "Undefined" "OverrideRootScale" null null))
  (`ProjectileMovementComponent.SetVelocityInLocalSpace` (`/Game/Assets/Characters/AI/BP_Bullet_AB.ProjectileMovement` _returnvalue) (+ (`self.GetVelocity` _returnvalue) (`self.ProjectileVelocity`))))

(fn `UpdateWalkSpeed`
  (params (NewWalkSpeed :type "Float (double-precision)"))
  (set `CharacterMovementComponent.MaxWalkSpeed` NewWalkSpeed (`self.CharacterMovement`)))

(fn `UserConstructionScript`)