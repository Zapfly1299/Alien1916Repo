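; AI controller for soldier enemies that runs BT_Soldier_AB on possession and feeds it player sightings.
; AI perception writes HasLineOfSight and EnemyActor to the blackboard; any other update starts a timer that clears both.
; The timer-cancel node is unwired, so regaining sight leaves a pending clear running.
; ShootOrder fires SoldierShoot on the last BP_Soldier_AB found at BeginPlay, rather than the possessed pawn.
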(event `self.OnPossess`
  (params (PossessedPawn :type "Pawn Object Reference"))
  (`self.RunBehaviorTree` "/Game/Assets/Characters/AI/BT_Soldier_AB.BT_Soldier_AB"))

(event `self.AIPerception.OnTargetPerceptionUpdated`
  (params (Actor :type "Actor Object Reference") (Stimulus :type "AIStimulus Structure"))
  (bind _blackboard (`self.Blackboard`))
  (if (and (`self.ActorHasTag` Actor "Player") (`.bSuccessfullySensed` (break `AIStimulus` Stimulus)))
    (`BlackboardComponent.SetValueAsBool` _blackboard (`self.HasLineOfSight`) true)
    (`BlackboardComponent.SetValueAsObject` _blackboard (`self.EnemyActor`) Actor)
    (else
      (bind _returnvalue (`KismetSystemLibrary.K2_SetTimerDelegate` (delegate `Start Enemy Timer`) (`self.Line of Sight Timer`)))
      (set `self.EnemyTimer` _returnvalue))))

(event `Start Enemy Timer`
  (bind _blackboard (`self.Blackboard`))
  (`BlackboardComponent.SetValueAsBool` _blackboard (`self.HasLineOfSight`) false)
  (`BlackboardComponent.SetValueAsObject` _blackboard (`self.EnemyActor`) null))

(event `ShootOrder`
  (`/Game/Assets/Characters/AI/BP_Soldier_AB.SoldierShoot` (`self.BP_Soldier_AB`)))

(event `self.ReceiveBeginPlay`
  (bind _outactors (`GameplayStatics.GetAllActorsOfClass` "/Game/Assets/Characters/AI/BP_Soldier_AB.BP_Soldier_AB_C"))
  (for _array_element _outactors
    (set `self.BP_Soldier_AB` _array_element)))

(fn `UserConstructionScript`)