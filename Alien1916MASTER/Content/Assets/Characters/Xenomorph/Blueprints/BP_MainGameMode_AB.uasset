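; Game mode Blueprint that creates the player HUD and drives its elapsed-time display.
; On BeginPlay it adds an MC_UI_Widget to the viewport for player controller 0 and starts a looping one-second timer on UITimer.
; UITimer increments CurrentTime, formats it as minutes and zero-padded seconds via a Timespan, and pushes the text to the HUD's UpdateTimer.
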(event `self.ReceiveBeginPlay`
  (bind _returnvalue (`|CreateWidget` "/Game/Assets/UI/MC_UI_Widget.MC_UI_Widget_C" (`GameplayStatics.GetPlayerController` 0)))
  (bind _output_get (set `self.PlayerHUDWidget` _returnvalue))
  (`UserWidget.AddToViewport` _output_get 0)
  (`KismetSystemLibrary.K2_SetTimer` null "UITimer" 1.0 true))

(fn `UITimer`
  (bind _result (`/Engine/EditorBlueprintResources/StandardMacros.IncrementFloat` (`self.CurrentTime`))
    (:`  `
      (bind (_returnvalue_days _returnvalue_hours _returnvalue_minutes _returnvalue_seconds) (`KismetMathLibrary.BreakTimespan` (`KismetMathLibrary.FromSeconds` _result)))
      (if (< _returnvalue_seconds 10)
        (set `self.NewTime` (`|FormatText` "{minute}:0{seconds}" _returnvalue_minutes _returnvalue_seconds))
        (else
          (set `self.NewTime` (`|FormatText` "{minute}:{seconds}" _returnvalue_minutes _returnvalue_seconds))))
      (`/Game/Assets/UI/MC_UI_Widget.UpdateTimer` (`self.PlayerHUDWidget`) (`self.NewTime`)))))

(fn `UserConstructionScript`)