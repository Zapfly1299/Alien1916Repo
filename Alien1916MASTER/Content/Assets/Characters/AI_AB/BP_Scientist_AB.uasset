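; BP_Scientist_AB is an AI character that can shoot at the player and take damage.
; BeginPlay sets two patrol points via opposite navigation raycasts, built from the mesh's forward vector rather than its location.
; SoldierShoot spawns a BP_Bullet_AB aimed at the player with fixed pitch and yaw offsets, then sets its velocity.
; Damage lowers and prints Health, destroying the actor on a hit after Health is negative; UpdateWalkSpeed sets movement speed.
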(event `self.ReceiveBeginPlay`
  (bind _hitlocation (`NavigationSystemV1.NavigationRaycast` (`SceneComponent.GetForwardVector` (`self.Mesh`)) (+ (`SceneComponent.GetForwardVector` (`self.Mesh`)) (0.0 1000.0 0.0)) null null))
  (set `self.PatrolPointOne` _hitlocation)
  (bind _hitlocation_2 (`NavigationSystemV1.NavigationRaycast` (`SceneComponent.GetForwardVector` (`self.Mesh`)) (+ (`SceneComponent.GetForwardVector` (`self.Mesh`)) (0.0 -1000.0 0.0)) null null))
  (set `self.PatrolPointTwo` _hitlocation_2))

(event `SoldierShoot`
  (bind _shootlocation (`self.ShootLocation`))
  (bind (_returnvalue_roll _returnvalue_pitch _returnvalue_yaw) (`KismetMathLibrary.BreakRotator` (`KismetMathLibrary.FindLookAtRotation` (`SceneComponent.K2_GetComponentLocation` _shootlocation) (`self.K2_GetActorLocation` (`GameplayStatics.GetPlayerPawn` 0)))))
  ;[1 1 1] Enemy Shooting At Player
  (bind _returnvalue (`|SpawnActorFromClass` "/Game/Assets/Characters/AI_AB/BP_Bullet_AB.BP_Bullet_AB_C" (`KismetMathLibrary.MakeTransform` (`SceneComponent.K2_GetComponentLocation` _shootlocation) (`KismetMathLibrary.MakeRotator` _returnvalue_roll (- _returnvalue_pitch 20.0) (- _returnvalue_yaw 35.0))) "Undefined" "OverrideRootScale" null null))
  (`ProjectileMovementComponent.SetVelocityInLocalSpace` (`/Game/Assets/Characters/AI_AB/BP_Bullet_AB.ProjectileMovement` _returnvalue) (+ (`self.GetVelocity` _returnvalue) (`self.ProjectileVelocity`))))

(event `self.ReceiveAnyDamage`
  (params (Damage :type "Float (single-precision)") (DamageType :type "DamageType Object Reference") (InstigatedBy :type "Controller Object Reference") (DamageCauser :type "Actor Object Reference"))
  ;[1 1 1] Take Damage
  (if (>= (`self.Health`) 0.0)
    (set `self.Health` (- (`self.Health`) Damage))
    (`KismetSystemLibrary.PrintString` (`KismetStringLibrary.Conv_DoubleToString` (`self.Health`)))
    (else
      (`self.K2_DestroyActor`))))

(fn `UpdateWalkSpeed`
  (params (NewWalkSpeed :type "Float (double-precision)"))
  (set `CharacterMovementComponent.MaxWalkSpeed` NewWalkSpeed (`self.CharacterMovement`)))

(fn `UserConstructionScript`)