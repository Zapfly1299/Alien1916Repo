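; AI controller for the scientist NPC that runs its behavior tree and feeds it patrol and enemy data through the Blackboard.
; On possession, navigation raycasts along roughly ±Y set two patrol points, the first from the pawn and the second from the controller.
; Perception sets line of sight and enemy on sensing BP_PhyCharTest_MJB, but never clears them.
; BeginPlay stores the last scientist found in the level, not specifically its own pawn.
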(event `self.OnPossess`
  (params (PossessedPawn :type "Pawn Object Reference"))
  (bind _returnvalue (`self.K2_GetActorLocation`))
  (bind _returnvalue_2 (`self.K2_GetActorLocation` PossessedPawn))
  (bind _blackboard (`self.Blackboard`))
  ;[1 1 1] Possession at start of game
  (`self.RunBehaviorTree` "/Game/Assets/Characters/AI_AB/BT_Scientist_AB.BT_Scientist_AB")
  (bind _hitlocation (`NavigationSystemV1.NavigationRaycast` _returnvalue_2 (+ _returnvalue_2 (+ (`self.GetActorForwardVector` PossessedPawn) (0.0 1000.0 0.0))) null null))
  (`BlackboardComponent.SetValueAsVector` _blackboard (`self.PatrolLocationOne`) _hitlocation)
  (bind _hitlocation_2 (`NavigationSystemV1.NavigationRaycast` _returnvalue (+ _returnvalue (+ (`self.GetActorForwardVector`) (0.0 -1000.0 0.0))) null null))
  (`BlackboardComponent.SetValueAsVector` _blackboard (`self.PatrolLocationTwo`) _hitlocation_2))

(event `self.AIPerception.OnTargetPerceptionUpdated`
  (params (Actor :type "Actor Object Reference") (Stimulus :type "AIStimulus Structure"))
  (bind _blackboard (`self.Blackboard`))
  ;[1 1 1] Line of sight and enemy identification
  (cast `/Game/Assets/Characters/Xenomorph/Blueprints/BP_PhyCharTest_MJB` Actor)
  (if (`.bSuccessfullySensed` (break `AIStimulus` Stimulus))
    (`BlackboardComponent.SetValueAsBool` _blackboard (`self.HasLineOfSight`) true)
    (`BlackboardComponent.SetValueAsObject` _blackboard (`self.EnemyActor`) Actor)))

(event `self.ReceiveBeginPlay`
  ;[1 1 1] Setting itself as a variable for BB purposes
  (bind _outactors (`GameplayStatics.GetAllActorsOfClass` "/Game/Assets/Characters/AI_AB/BP_Scientist_AB.BP_Scientist_AB_C"))
  (for _array_element _outactors
    (set `self.BP_Scientist_AB` _array_element)))

(fn `UserConstructionScript`)